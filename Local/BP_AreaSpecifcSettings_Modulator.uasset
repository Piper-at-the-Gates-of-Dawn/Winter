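; Volume actor that overrides a named Ultra Dynamic Sky area-specific setting while the player is inside its bounds.
; On BeginPlay, outside dedicated servers, it finds that entry by name, caches its defaults and enables overlap queries.
; UpdateAreaSettings applies custom values on player entry and restores defaults on exit.
; A delayed spawn check (`>= 0`, so always true) applies custom values; a looping timer also targets UpdateAreaSettings by name.
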(event OnComponentBeginOverlap(Modulator_Bounds)
  (params (OverlappedComponent :type Primitive%20Component%20Object%20Reference) (OtherActor :type Actor%20Object%20Reference) (OtherComp :type Primitive%20Component%20Object%20Reference) (OtherBodyIndex :type Integer) (bFromSweep :type Boolean) (SweepResult :type Hit%20Result%20Structure%20%28by%20ref%29))
  ;[1 1 1] While within "Modulator_Bounds", the AreaSpecificSettings named by AreaSettingsToUse, will be overwritten by the "CustomArea..." settings.
  (if (== (Utilities|GetClass OtherActor) "/Game/Characters/BasePlayerChar.BasePlayerChar_C")
    (CallFunction|UpdateAreaSettings true)))

(event OnComponentEndOverlap(Modulator_Bounds)
  (params (OverlappedComponent :type Primitive%20Component%20Object%20Reference) (OtherActor :type Actor%20Object%20Reference) (OtherComp :type Primitive%20Component%20Object%20Reference) (OtherBodyIndex :type Integer))
  ;[1 1 1] While within "Modulator_Bounds", the AreaSpecificSettings named by AreaSettingsToUse, will be overwritten by the "CustomArea..." settings.
  (if (== (Utilities|GetClass OtherActor) "/Game/Characters/BasePlayerChar.BasePlayerChar_C")
    (CallFunction|UpdateAreaSettings false)))

(event EventBeginPlay
  (Utilities|FlowControl|Sequence
    (:then_0
      (if (not (Networking|IsDedicatedServer))
        ;[1 1 1] Get the Skybox
        (bind _outactors (Actor|GetAllActorsOfClass "/Game/Marketplace/UltraDynamicSky/Blueprints/Ultra_Dynamic_Sky_BP.Ultra_Dynamic_Sky_BP_C"))
        (Variables|Default|SetDynamicSky_Normal (Utilities|Array|Get(acopy) _outactors))
        ;[1 1 1] Look through the Skybox's "AreaSpecificSettings" array and grab the setting matching the name of "Area Setting to Use"
        (bind (_array_element _array_index) (Utilities|Array|ForEachLoopwithBreak (Variables|/Game/Marketplace/UltraDynamicSky/Blueprints/Ultra_Dynamic_Sky_BP.Ultra_Dynamic_Sky_BP_C|GetAreaSpecificSettings (Variables|Default|GetDynamicSky_Normal)) :!label _label)
          (:LoopBody
            (if (Utilities|Enum|Equal(Enum) (.name (Utilities|Struct|BreakSkyCurveSet _array_element)) (Variables|Default|GetAreaSettingsToUse))
              (Variables|Default|SetAreaSpecificSettingsIndex _array_index)
              (Variables|Default|Setfound true)
              (Variables|Default|SetDefaultAreaVolume (.Volume (Utilities|Struct|BreakSkyCurveSet _array_element)))
              (Variables|Default|SetDefaultAreaLocation (.Center (Utilities|Struct|BreakSkyCurveSet _array_element)))
              (Variables|Default|SetDefaultAreaRadius (.radius (Utilities|Struct|BreakSkyCurveSet _array_element)))
              (Variables|Default|SetDefaultAreaFadeExponent (.fadeExponent (Utilities|Struct|BreakSkyCurveSet _array_element)))
              (Variables|Default|SetDefaultAreaPriority (.Priority (Utilities|Struct|BreakSkyCurveSet _array_element)))
              (goto _label Break)))
          (:Completed
            (if (Variables|Default|Getfound)
              (Collision|SetCollisionEnabled (Variables|Default|GetModulator_Bounds) "QueryOnly"))))))
    (:then_1
      ;[1 1 1] Check If Player Spawned In Bounds. If so, run update as if trigger was entered.
      (Utilities|FlowControl|Delay 1.0)
      (if (>= (Utilities|Array|Length (Collision|GetOverlappingActors (Variables|Default|GetModulator_Bounds) "/Game/Characters/BasePlayerChar.BasePlayerChar_C" :!class /Script/Engine.PrimitiveComponent)) 0)
        (Development|PrintString "PlayerSpawned In Bounds")
        ;[1 1 1] While within "Modulator_Bounds", the AreaSpecificSettings named by AreaSettingsToUse, will be overwritten by the "CustomArea..." settings.
        (CallFunction|UpdateAreaSettings true)
        (else
          (Development|PrintString "Hello"))))
    (:then_2
      (Utilities|Time|SetTimerbyFunctionName self "UpdateAreaSettings" 1e+01 true))))

(fn ConstructionScript)

(fn UpdateAreaSettings
  (params (Entered :type Boolean))
  ;[1 1 1] Comment
  (Development|PrintString "Update Area Settings")
  (if (Variables|Default|Getfound)
    (Default|SetAreaSpecificParams (Variables|Default|GetDynamicSky_Normal) (Variables|Default|GetAreaSpecificSettingsIndex) (Utilities|Struct|MakeEnvironmentArea (select Entered (Variables|Dungeon|GetCustomAreaLocation) (Variables|Default|GetDefaultAreaLocation)) (select Entered (Variables|Dungeon|GetCustomAreaVolume) (Variables|Default|GetDefaultAreaVolume)) (select Entered (Variables|Dungeon|GetCustomAreaPriority) (Variables|Default|GetDefaultAreaPriority)) (select Entered (Variables|Dungeon|GetCustomAreaRadius) (Variables|Default|GetDefaultAreaRadius)) (select Entered (Variables|Dungeon|GetCustomAreaFadeExponent) (Variables|Default|GetDefaultAreaFadeExponent)) -1.0))))