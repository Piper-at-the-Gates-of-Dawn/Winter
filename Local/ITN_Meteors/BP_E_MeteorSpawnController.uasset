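; Server-driven controller that randomly triggers meteor showers.
; A looping timer rolls a spawn chance that resets after each shower, then climbs once a cooldown runs out.
; Each shower spawns a randomized count of BP_E_MeteorProjectile actors inside a box along an arrow's rotation, with random delays and velocity offsets.
; It passes spawner height to each particle material for sky fading and increments translucency sort priority.
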(event Custom|SpawnMeteorShower
  (bind _meteorshowerrandomamount (Variables|Default|GetMeteorShowerRandomAmount))
  (bind _output_get (Variables|Default|SetMeteorShowerTempMaxCount (+ (Variables|Default|GetMeteorShowerMaxCount) (Math|Random|RandomIntegerinRange (* _meteorshowerrandomamount -1) _meteorshowerrandomamount))))
  (if (> _output_get (Variables|Default|GetMeteorShowerAmountSpawned)) :!label _label
    (bind _returnvalue (Game|SpawnActorfromClass "/Game/Mods/The_Isle_of_Tir-na-nOg/ITN_Meteors/BP_E_MeteorProjectile.BP_E_MeteorProjectile_C" (Math|Transform|MakeTransform (Class|FuncomGenericLibrary|GetRandomPointinBox (Variables|Default|GetBox)) (Transformation|GetWorldRotation (Variables|Default|GetArrow)) "1.000000,1.000000,1.000000") "AlwaysSpawn" self (Math|Vector|MakeVector (Math|Random|RandomFloatinRange 0.06 -0.06) (Math|Random|RandomFloatinRange 0.06 -0.06) (Math|Random|RandomFloatinRange 0.06 -0.06)) 0))
    (Utilities|FlowControl|Delay (Math|Random|RandomFloatinRange 0.05 1.0))
    (bind _output_get_2 (Variables|Default|SetMeteorShowerAmountSpawned (+ (Variables|Default|GetMeteorShowerAmountSpawned) 1)))
    (Utilities|IsValid (Variables|/Game/Mods/The_Isle_of_Tir-na-nOg/ITN_Meteors/BP_E_MeteorProjectile.BP_E_MeteorProjectile_C|GetParticleSystem _returnvalue)
      (:Is%20Valid
        ;[1 1 1] Give Height information about spawner to material to do fadeout into sky
        (bind _returnvalue_2 (Rendering|Material|CreateDynamicMaterialInstance (Variables|/Game/Mods/The_Isle_of_Tir-na-nOg/ITN_Meteors/BP_E_MeteorProjectile.BP_E_MeteorProjectile_C|GetParticleSystem _returnvalue) 0 (Rendering|Material|GetMaterial (Variables|/Game/Mods/The_Isle_of_Tir-na-nOg/ITN_Meteors/BP_E_MeteorProjectile.BP_E_MeteorProjectile_C|GetParticleSystem _returnvalue) 0) :!class /Script/Engine.PrimitiveComponent))
        (Rendering|Material|SetScalarParameterValue _returnvalue_2 "spawn_height" (.z (Transformation|GetActorLocation self)) :!class /Script/Engine.MaterialInstanceDynamic)
        (Rendering|SetTranslucentSortPriority (Variables|/Game/Mods/The_Isle_of_Tir-na-nOg/ITN_Meteors/BP_E_MeteorProjectile.BP_E_MeteorProjectile_C|GetParticleSystem _returnvalue) _output_get_2)
        (goto _label))
      (:Is%20Not%20Valid
        (goto _label)))
    (else
      (Variables|Default|SetMeteorCooldown 5)
      (Variables|Default|SetChanceToTriggerMeteor 0)
      (Variables|Default|SetMeteorShowerAmountSpawned 0))))

(event Custom|CheckIfShouldSpawnMeteor
  (if (and (< (Math|Random|RandomIntegerinRange 0 100) (Variables|Default|GetChanceToTriggerMeteor)) (<= (Variables|Default|GetMeteorCooldown) 0))
    (CallFunction|SpawnMeteorShower)
    (else
      (bind _result (Math|Integer|DecrementInt (Variables|Default|GetMeteorCooldown))
        (:%20%20
          (if (<= _result 0)
            (Variables|Default|SetChanceToTriggerMeteor (+ (Variables|Default|GetChanceToTriggerMeteor) (Variables|Default|GetChanceIncement)))))))))

(event EventBeginPlay
  (if (Networking|IsServer)
    (Utilities|Time|SetTimerbyEvent (delegate Custom|CheckIfShouldSpawnMeteor) (Variables|Default|GetChance%20to%20Spawn%20Timer) true)))

(fn ConstructionScript)