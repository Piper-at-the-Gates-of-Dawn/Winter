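; Meteor projectile that flies on controller-supplied velocity rotated to its orientation, damaging what it overlaps and whatever surrounds its impact.
; On stop, non-dedicated instances play impact effects and fade sound and light.
; The server spawns a ground-traced BP_E_Grounded harvestable, excludes it from paired health and explosive radial damage, then sets a lifespan.
; A BeginPlay hack removes the light when the local player is inside climbing-blocking volumes (dungeons).
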(event OnProjectileStop(ProjectileMovement)
  (params (ImpactResult :type Hit%20Result%20Structure%20%28by%20ref%29))
  ;[1 0.6413 0.1882] OnProjectileStopped (On Impact)
  (Utilities|FlowControl|Sequence
    (:then_0
      ;;[0.02499 0.09524 0.16] Handle Impact Sound
      (if (not (Networking|IsDedicatedServer))
        (Class|ConanAudioComponent|FadeOut (Variables|Default|GetConanAudio) 1.0 0.0)
        (Class|DreamworldBlueprints|PlaySoundatLocation (Variables|Default|GetAudio_Impact) (Transformation|GetActorLocation))))
    (:then_1
      ;;[0.02499 0.09524 0.16] Handle Impact Effects
      (if (not (Networking|IsDedicatedServer))
        (Components|Activation|Deactivate (Variables|Default|GetParticleSystem))
        (Components|DestroyComponent (Variables|Default|GetP_meteortrail_glow))
        (Effects|SpawnEmitteratLocation "/Game/Mods/The_Isle_of_Tir-na-nOg/ITN_Meteors/P_E_meteor_impact.P_E_meteor_impact" (Transformation|GetActorLocation))
        (bind _fade (Timeline|light_fadeout Play)
          (:Update
            (Rendering|Components|Light|SetIntensity (Variables|Default|GetPointLight) _fade)))))
    (:then_2
      ;;[0.02499 0.09524 0.16] Handle Spawn Harvestable
      (if (Networking|IsServer)
        (bind _groundedactor (CallFunction|SpawnGroundedActor))))
    (:then_3
      ;;[0.02499 0.09524 0.16] Handle Impact Damage
      (CallFunction|DoDamage _groundedactor))
    (:then_4
      ;;[0.02499 0.09524 0.16] Handle Death
      (if (Networking|IsServer)
        (Actor|SetLifeSpan (Variables|Default|GetOnImpactLifeSpan))))))

(event OnComponentActivated(ProjectileMovement)
  (params (Component :type Actor%20Component%20Object%20Reference) (bReset :type Boolean))
  (bind _projectilemovement (Variables|Default|GetProjectileMovement))
  ;[1 1 1] Set Orientation and direction from Controller
  (Variables|/Script/Engine.MovementComponent|SetVelocity _projectilemovement (Math|Vector|RotateVector (+ (Variables|Default|Getcontroller_velocity) (Variables|/Script/Engine.MovementComponent|GetVelocity _projectilemovement)) (Transformation|GetActorRotation))))

(event OnComponentBeginOverlap(BoxCollision)
  (params (OverlappedComponent :type Primitive%20Component%20Object%20Reference) (OtherActor :type Actor%20Object%20Reference) (OtherComp :type Primitive%20Component%20Object%20Reference) (OtherBodyIndex :type Integer) (bFromSweep :type Boolean) (SweepResult :type Hit%20Result%20Structure%20%28by%20ref%29))
  (bind _impactpoint (Collision|BreakHitResult SweepResult))
  (bind _self self)
  (bind _array (Utilities|Array|MakeArray _self))
  ;[1 0.035 0.035] Damage on Overlap
  (|ApplyRadialDamagewithFalloffAsync 1e+02 0.0 _impactpoint 125.0 125.0 1.0 "/Game/Systems/Progression/DmgTypeHealth_BP.DmgTypeHealth_BP_C" _array _self 0 "ECC_Visibility"
    (:then
      (|ApplyRadialDamagewithFalloffAsync 1e+02 0.0 _impactpoint 128.0 125.0 2.0 "/Game/Systems/Combat/Dmg_Explosive.Dmg_Explosive_C" _array _self 0 "ECC_Visibility"))))

(event Custom|DoDamage
  (params (GroundedProjectileToIgnore :type Actor%20Object%20Reference))
  (bind _self self)
  (bind _basedamage (Variables|DamageConfig|GetBaseDamage))
  (bind _array (Utilities|Array|MakeArray GroundedProjectileToIgnore _self))
  ;[0.62 0 0] Damage
  (if (Networking|IsServer)
    (|ApplyRadialDamagewithFalloffAsync _basedamage 0.0 (Transformation|GetActorLocation) 2056.0 2056.0 1.0 "/Game/Systems/Progression/DmgTypeHealth_BP.DmgTypeHealth_BP_C" _array self 0 "ECC_Visibility"
      (:then
        (|ApplyRadialDamagewithFalloffAsync (* _basedamage 1e+02) 0.0 (Transformation|GetActorLocation) 2056.0 2056.0 2.0 "/Game/Systems/Combat/Dmg_Explosive.Dmg_Explosive_C" _array self 0 "ECC_Visibility")))))

(event Custom|MulticastDebugSpheres
  (bind _returnvalue (Transformation|GetActorLocation))
  ;[0.62 0 0] Damage
  (Rendering|Debug|DrawDebugSphere _returnvalue 125.0 30 "(R=0.620000,G=0.000000,B=0.000000,A=1.000000)" 1e+01 2e+01)
  (Rendering|Debug|DrawDebugSphere _returnvalue 125.0 30 "(R=1.000000,G=0.641254,B=0.188168,A=1.000000)" 1e+01 2e+01))

(event EventBeginPlay
  (bind _conanaudio (Variables|Default|GetConanAudio))
  ;[1 1 1] Hacky Fix for Lights inside dungeons
  (Utilities|IsValid _conanaudio
    (:Is%20Valid
      (Class|ConanAudioComponent|Play _conanaudio 0.0))
    (:Is%20Not%20Valid
      _))
  (if (not (Networking|IsDedicatedServer))
    (bind _asconan_character (Utilities|Casting|CastToConanCharacter (Game|Player|GetPlayerPawn 0)))
    (if (> (Variables|/Script/ConanSandbox.ConanCharacter|GetClimbingBlockingVolumeCount _asconan_character) 0)
      (Components|DestroyComponent (Variables|Default|GetPointLight)))))

(fn ConstructionScript)

(fn SpawnGroundedActor
  (bind _returnvalue (Transformation|GetActorTransform))
  (bind _returnvalue_2 (Transformation|GetActorTransform))
  (bind _location (Math|Transform|BreakTransform _returnvalue_2))
  (bind (_location_2 _rotation _scale) (Math|Transform|BreakTransform _returnvalue))
  ;[0.62 0 0] Make sure projectile gets embedded in the ground.
  (bind (_outhit _returnvalue_3) (Collision|LineTraceByChannel _location (+ _location (* "0, 0,-1.000000" 2e+02)) "TraceTypeQuery1" false 0 "None"))
  (bind _returnvalue_4 (Game|SpawnActorfromClass "/Game/Mods/The_Isle_of_Tir-na-nOg/ITN_Meteors/BP_E_Grounded.BP_E_Grounded_C" (select _returnvalue_3 (Math|Transform|MakeTransform (.Location (Collision|BreakHitResult _outhit)) _rotation _scale) (Transformation|GetActorTransform)) "AlwaysSpawn" 0 0))
  (Default|Initialize _returnvalue_4)
  (return _returnvalue_4))