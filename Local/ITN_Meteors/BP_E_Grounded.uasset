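; Grounded meteor actor that only explosive radial damage breaks, leaving a non-respawning core resource node.
; On death it multicasts a shatter destructible effect, and the server spawns the replicated BP_ResourceActor.
; Weapon hits show the attacker a HUD notification, and a server timer despawns it after just under four hours.
; The mesh is set via OnRep, and a health-based emissive crack effect is defined but not called here.
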(event Custom|Initialize
  ;[1 0.6413 0.1882] Initialize
  (Components|StaticMesh|SetStaticMesh (Variables|Default|GetStaticMesh) (Variables|Default|GetStaticMeshToShow)))

(event Custom|MulticastOnDamaged
  (params (Health%25 :type Integer))
  ;[1 0.6413 0.1882] Cracks material effect.
  (Rendering|Material|SetVectorParameterValueonMaterials (Variables|Default|GetStaticMesh) "EmissiveChoke" (Math|Conversions|ToVector(LinearColor) (select (<= Health%25 25) "(R=0.970000,G=0.970000,B=0.970000,A=1.000000)" (select (<= Health%25 50) "(R=0.830000,G=0.830000,B=0.830000,A=1.000000)" (select (<= Health%25 75) "(R=0.715000,G=0.715000,B=0.715000,A=1.000000)" (select (<= Health%25 100) "(R=0.640000,G=0.640000,B=0.640000,A=1.000000)" "")))))))

(event Custom|Despawn
  ;[0.02499 0.09524 0.16] Handle Despawn
  (Actor|DestroyActor))

(event Custom|OnDeath
  ;[0.62 0 0] Death
  (if (Networking|IsServer)
    (bind _returnvalue (Game|SpawnActorfromClass "/Game/Systems/Survival/Gathering/BP_ResourceActor.BP_ResourceActor_C" (Transformation|GetActorTransform) "AlwaysSpawn" 0 (Variables|Default|GetCoreVisualMesh) 0 false -1 "Resource" (Variables|Default|GetCoreDestructibleMesh) "0.000000,0.000000,0.000000" 0 0 false))
    (Networking|SetReplicates _returnvalue true)
    (Actor|DestroyActor)))

(event Custom|MulticastOnDeath
  ;[1 0.6413 0.1882] Multicast destruction effect.
  (if (not (Networking|IsDedicatedServer))
    (Game|SpawnActorfromClass "/Game/Systems/Survival/Gathering/Gathering_v2/ResourceDestructibleMeshActor.ResourceDestructibleMeshActor_C" (Transformation|GetActorTransform) "AlwaysSpawn" 0 (Variables|Default|GetShatterDestructibleMesh) 0 false)))

(event EventBeginPlay
  ;[0.02499 0.09524 0.16] Handle Despawn
  (if (Networking|IsServer)
    (Utilities|Time|SetTimerbyEvent (delegate Custom|Despawn) 1.4e+04) ; A little bit less than 4 hours.
  ))

(event Game|Damage|EventRadialDamage
  (params (DamageReceived :type Float%20%28single-precision%29) (DamageType :type Damage%20Type%20Object%20Reference) (Origin :type Vector :default "0, 0, 0") (HitInfo :type Hit%20Result%20Structure%20%28by%20ref%29) (InstigatedBy :type Controller%20Object%20Reference) (DamageCauser :type Actor%20Object%20Reference))
  ;[1 0.6413 0.1882] Handle Damage
  (Utilities|And+Branch (Utilities|DoesObjectImplementInterface DamageCauser "/Game/Items/Weapons/Orbs/IsOrbEffectInterface.IsOrbEffectInterface_C") (Utilities|DoesObjectImplementInterface DamageCauser "/Game/Systems/SkySpawning/IsMeteorProjectileInterface.IsMeteorProjectileInterface_C")
    (:False
      (Utilities|And+Branch (> DamageReceived 0.0) (== (Utilities|GetClass DamageType) "/Game/Systems/Combat/Dmg_Explosive.Dmg_Explosive_C")
        (:True
          (CallFunction|MulticastonDeath)
          (CallFunction|OnDeath))))))

(event Game|Damage|EventAnyDamage
  (params (Damage :type Float%20%28single-precision%29) (DamageType :type Damage%20Type%20Object%20Reference) (InstigatedBy :type Controller%20Object%20Reference) (DamageCauser :type Actor%20Object%20Reference) (DamageEventID :type Integer))
  ;[1 1 1] Show FIFO if you attack it with something else than explosives
  (if (Utilities|DoesObjectImplementInterface DamageCauser "/Game/Items/Weapons/BaseWeaponInterface.BaseWeaponInterface_C")
    (bind _asconan_character (Utilities|Casting|CastToConanCharacter (Pawn|GetControlledPawn InstigatedBy)))
    (Class|ConanCharacter|ClientHUDShowNotification _asconan_character (Variables|Default|GetFIFO) false)))

(fn ConstructionScript)

(fn OnRepHitPoints)

(fn OnRepStaticMeshtoShow
  (Components|StaticMesh|SetStaticMesh (Variables|Default|GetStaticMesh) (Variables|Default|GetStaticMeshToShow)))