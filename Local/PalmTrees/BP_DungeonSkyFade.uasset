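; Dungeon trigger that changes Ultra Dynamic Sky's area-specific lighting while the local player is inside its box.
; On BeginPlay it finds the sky area named by AreaToHijack, caches its defaults and enables box queries.
; Overlap moves that area to the dungeon's center, volume, radius, fade and priority, restoring them on exit.
; ForceDark also swaps in a prebuilt copy with overridden light, fog, cloud-wisp and scattering curves.
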(event OnComponentBeginOverlap(Box)
  (params (OverlappedComponent :type Primitive%20Component%20Object%20Reference) (OtherActor :type Actor%20Object%20Reference) (OtherComp :type Primitive%20Component%20Object%20Reference) (OtherBodyIndex :type Integer) (bFromSweep :type Boolean) (SweepResult :type Hit%20Result%20Structure%20%28by%20ref%29))
  (Utilities|IsPlayer OtherActor
    (:True
      (CallFunction|MoveArea true)
      (Development|PrintString "Entered"))))

(event OnComponentEndOverlap(Box)
  (params (OverlappedComponent :type Primitive%20Component%20Object%20Reference) (OtherActor :type Actor%20Object%20Reference) (OtherComp :type Primitive%20Component%20Object%20Reference) (OtherBodyIndex :type Integer))
  (Utilities|IsPlayer OtherActor
    (:True
      (CallFunction|MoveArea false)
      (Development|PrintString "Exited"))))

(event EventBeginPlay
  (if (Networking|IsDedicatedServer)
    _
    (else
      _))
  (bind _outactors (Actor|GetAllActorsOfClass "/Game/Marketplace/UltraDynamicSky/Blueprints/Ultra_Dynamic_Sky_BP.Ultra_Dynamic_Sky_BP_C"))
  (bind _output_get (Variables|Default|SetDynamicSky_Normal (Utilities|Array|Get(acopy) _outactors)))
  (Utilities|IsValid _output_get
    (:Is%20Valid
      (bind (_array_element _array_index) (Utilities|Array|ForEachLoopwithBreak (Variables|/Game/Marketplace/UltraDynamicSky/Blueprints/Ultra_Dynamic_Sky_BP.Ultra_Dynamic_Sky_BP_C|GetAreaSpecificSettings (Variables|Default|GetDynamicSky_Normal)) :!label _label)
        (:LoopBody
          (if (Utilities|Enum|Equal(Enum) (.name (Utilities|Struct|BreakSkyCurveSet _array_element)) (Variables|Default|GetAreaToHijack))
            (Variables|Default|SetAreaSpecificSettingsIndex _array_index)
            (Variables|Default|SetFound true)
            (Variables|Default|SetDefaultVolume (.Volume (Utilities|Struct|BreakSkyCurveSet _array_element)))
            (Variables|Default|SetDefaultLocation (.Center (Utilities|Struct|BreakSkyCurveSet _array_element)))
            (Variables|Default|SetDefaultRadius (.radius (Utilities|Struct|BreakSkyCurveSet _array_element)))
            (Variables|Default|SetDefaultFadeExponent (.fadeExponent (Utilities|Struct|BreakSkyCurveSet _array_element)))
            (Variables|Default|SetDefaultPriority (.Priority (Utilities|Struct|BreakSkyCurveSet _array_element)))
            (goto _label Break)))
        (:Completed
          (if (Variables|Default|GetFound)
            (if (Variables|Default|GetForceDark)
              (PatchArray|BuildPatchArrays))
            (Collision|SetCollisionEnabled (Variables|Default|GetBox) "QueryOnly")))))))

(fn ConstructionScript)

(fn MoveArea
  (params (Entered :type Boolean))
  (PatchArray|PatchArray Entered)
  (Default|SetAreaSpecificParams (Variables|Default|GetDynamicSky_Normal) (Variables|Default|GetAreaSpecificSettingsIndex) (Utilities|Struct|MakeEnvironmentArea (select Entered (Variables|Dungeon|GetDungeonLocation) (Variables|Default|GetDefaultLocation)) (select Entered (Variables|Dungeon|GetDungeonVolume) (Variables|Default|GetDefaultVolume)) (select Entered (Variables|Dungeon|GetDungeonPriority) (Variables|Default|GetDefaultPriority)) (select Entered (Variables|Dungeon|GetDungeonRadius) (Variables|Default|GetDefaultRadius)) (select Entered (Variables|Dungeon|GetDungeonFadeExponent) (Variables|Default|GetDefaultFadeExponent)) -1.0)))

(fn PatchArray
  (params (Patch? :type Boolean))
  (if (Variables|Default|GetForceDark)
    (Utilities|Array|SetArrayElem (Variables|/Game/Marketplace/UltraDynamicSky/Blueprints/Ultra_Dynamic_Sky_BP.Ultra_Dynamic_Sky_BP_C|GetAreaSpecificSettings (Variables|Default|GetDynamicSky_Normal)) (Variables|Default|GetAreaSpecificSettingsIndex) (select Patch? (Variables|PatchArray|GetNewArray) (Variables|PatchArray|GetOldArray)))))

(fn BuildPatchArrays
  (bind _lightcurve (Variables|PatchArray|GetLightCurve))
  (Variables|PatchArray|SetOldArray (|Copy (Utilities|Array|Get(acopy) (Variables|/Game/Marketplace/UltraDynamicSky/Blueprints/Ultra_Dynamic_Sky_BP.Ultra_Dynamic_Sky_BP_C|GetAreaSpecificSettings (Variables|Default|GetDynamicSky_Normal)) (Variables|Default|GetAreaSpecificSettingsIndex))))
  (Variables|PatchArray|SetNewArray (Utilities|Struct|MakeSkyCurveSet (.name (Variables|PatchArray|GetOldArray)) (.horizoncolourcurve (Variables|PatchArray|GetOldArray)) (.zenithcolourcurve (Variables|PatchArray|GetOldArray)) (.cloudlightcolourcurve (Variables|PatchArray|GetOldArray)) (.clouddarkcolourcurve (Variables|PatchArray|GetOldArray)) (.suncolourcurve (Variables|PatchArray|GetOldArray)) (.shineintensitycurve (Variables|PatchArray|GetOldArray)) (.suncloudycolourcurve (Variables|PatchArray|GetOldArray)) (.starsintensitycurve (Variables|PatchArray|GetOldArray)) _lightcurve (.sunhighlightradiuscurve (Variables|PatchArray|GetOldArray)) (.nightfiltercurve (Variables|PatchArray|GetOldArray)) (Variables|PatchArray|GetFogCurve) (.fogstartdistcurve (Variables|PatchArray|GetOldArray)) (.fogcolouroverridecurve (Variables|PatchArray|GetOldArray)) (.volume (Variables|PatchArray|GetOldArray)) (.center (Variables|PatchArray|GetOldArray)) (.radius (Variables|PatchArray|GetOldArray)) (.fadeexponent (Variables|PatchArray|GetOldArray)) (.priority (Variables|PatchArray|GetOldArray)) (.fogfalloff (Variables|PatchArray|GetOldArray)) _lightcurve _lightcurve (.clouddensity (Variables|PatchArray|GetOldArray)) (.fogheightoffset (Variables|PatchArray|GetOldArray)) (.fogheightrelativetoplayer (Variables|PatchArray|GetOldArray)) (.rainstrength (Variables|PatchArray|GetOldArray)) "/Game/Marketplace/UltraDynamicSky/Materials/CloudWispsOpacityCurve.CloudWispsOpacityCurve" "/Game/Marketplace/UltraDynamicSky/Materials/DirectionalScatteringIntensityCurve.DirectionalScatteringIntensityCurve")))