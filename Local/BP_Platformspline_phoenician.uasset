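; Replicated moving platform with a multi-part skeletal character on master pose, carried along a target actor's spline.
; The main timeline sets the actor transform from spline distance; the server restarts runs after random delays via multicast, with run-counter OnReps for clients.
; TimelineAdjustments thresholds change play rates and drive a second timeline that rotates the platform.
; That local timeline is marked not fixed for replication, and location offsets are stored but never applied.
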(event Custom|MovePlatform
  (bind _targetsplineactor (Variables|Default|GetTargetSplineActor))
  (bind _relativearrowrotation (Variables|Default|GetRelativeArrowRotation))
  (bind _returnvalue (Actor|GetComponentbyClass _targetsplineactor "/Script/Engine.SplineComponent"))
  ;[1 1 1] Main Timeline
  (bind _movementtimeline (Timeline|Timeline_0 PlayFromStart)
    (:Update
      (if (Variables|Default|GetNoTimelineChecks)
        _
        (elif (Variables|Default|GetCompletedAllTimelineChecks)
          _
          (elif (> _movementtimeline (.timelinecheck (Utilities|Array|Get(acopy) (Variables|Default|GetTimelineAdjustments) (Variables|Default|GetTimelineCheckIndex))))
            (CallFunction|ApplyAdjustment)
            (bind _result (Math|Integer|IncrementInt (Variables|Default|GetTimelineCheckIndex))
              (:%20%20
                (Variables|Default|SetTimelineCheckIndex _result)
                (if (== (Utilities|Array|Length (Variables|Default|GetTimelineAdjustments)) (Variables|Default|GetTimelineCheckIndex))
                  (Variables|Default|SetCompletedAllTimelineChecks true)))))))
      (Transformation|SetActorTransform self (Math|Transform|MakeTransform (Spline|GetLocationatDistanceAlongSpline _returnvalue (* (Spline|GetSplineLength _returnvalue) _movementtimeline) "World") (Math|Rotator|MakeRotator (+ (.roll _relativearrowrotation) (.roll (Spline|GetRotationatDistanceAlongSpline _returnvalue (* (Spline|GetSplineLength _returnvalue) _movementtimeline) "World"))) (+ (.pitch _relativearrowrotation) (.pitch (Spline|GetRotationatDistanceAlongSpline _returnvalue (* (Spline|GetSplineLength _returnvalue) _movementtimeline) "World"))) (+ (.yaw _relativearrowrotation) (.yaw (Spline|GetRotationatDistanceAlongSpline _returnvalue (* (Spline|GetSplineLength _returnvalue) _movementtimeline) "World"))))))
      (if (Networking|IsServer)
        (Variables|Default|SetCurrentTimeLinePos _movementtimeline)))
    (:Finished
      (CallFunction|StopLocalTimeline)
      (Variables|Default|SetTimelineCheckIndex 0)
      (Variables|Default|SetCompletedAllTimelineChecks false)
      (Variables|Default|SetPreviousPlatformRotation "0, 0, 0")
      (Variables|Default|SetNewRotationOffset "0, 0, 0")
      (Components|Timeline|SetPlayRate (Variables|Default|GetTimeline_0) (Variables|Default|GetMainTimelinePlayRate))
      (Transformation|SetRelativeTransform (Variables|Default|GetPlatform) (Variables|Default|GetRelativePlatformTransform) false false)
      (Transformation|SetActorRotation self (Variables|Default|GetRelativeArrowRotation))
      (if (Networking|IsServer)
        (Utilities|FlowControl|Delay (Math|Random|RandomFloatinRange (Variables|Default|GetRandomDelayBeforeResetMin) (Variables|Default|GetRandomDelayBeforeResetMax)))
        (Variables|Default|SetCurrentTimeLinePos 0.0)
        (bind _output_get (Variables|Default|SetCurrentRunCounter (+ (Variables|Default|GetCurrentRunCounter) 1)))
        (CallFunction|MulticastStartMovePlatform _output_get)))))

(event Custom|StartLocalTimelineClient
  ;[1 0 0] NOT FIXED FOR REPLICATION: Platform Local Timeline Adjustments
  (Utilities|FlowControl|Sequence
    (:then_0
      (bind _newtrack_0 (Timeline|Timeline_1 SetNewTime)
        (:Update
          (Transformation|SetRelativeTransform (Variables|Default|GetPlatform) (Math|Transform|MakeTransform "0, 0, 0" (Math|Rotator|MakeRotator (.roll (Math|Interpolation|RInterpTo (Variables|Default|GetPreviousPlatformRotation) (Variables|Default|GetNewRotationOffset) _newtrack_0 1.0)) (.pitch (Math|Interpolation|RInterpTo (Variables|Default|GetPreviousPlatformRotation) (Variables|Default|GetNewRotationOffset) _newtrack_0 1.0)) (.yaw (Math|Interpolation|RInterpTo (Variables|Default|GetPreviousPlatformRotation) (Variables|Default|GetNewRotationOffset) _newtrack_0 1.0))) (Transformation|GetWorldScale (Variables|Default|GetPlatform))) false false)
          (if (Networking|IsServer)
            (Variables|Default|SetCurrentLocalTimelinePosition _newtrack_0)))
        (:Finished
          (Variables|Default|SetPreviousPlatformRotation (.Rotation (Math|Transform|BreakTransform (Math|Transform|MakeTransform "0, 0, 0" (Math|Rotator|MakeRotator (.roll (Math|Interpolation|RInterpTo (Variables|Default|GetPreviousPlatformRotation) (Variables|Default|GetNewRotationOffset) _newtrack_0 1.0)) (.pitch (Math|Interpolation|RInterpTo (Variables|Default|GetPreviousPlatformRotation) (Variables|Default|GetNewRotationOffset) _newtrack_0 1.0)) (.yaw (Math|Interpolation|RInterpTo (Variables|Default|GetPreviousPlatformRotation) (Variables|Default|GetNewRotationOffset) _newtrack_0 1.0))) (Transformation|GetWorldScale (Variables|Default|GetPlatform)))))))))
    (:then_1
      (Timeline|Timeline_1 Play))))

(event Custom|Apply%20adjustment
  (bind _timelinecheckindex (Variables|Default|GetTimelineCheckIndex))
  (bind _timelineadjustments (Variables|Default|GetTimelineAdjustments))
  (bind _relativeplatformtransform (Variables|Default|GetRelativePlatformTransform))
  (bind _item (Utilities|Array|Get(acopy) _timelineadjustments _timelinecheckindex))
  (bind (_roll _pitch _yaw) (Math|Rotator|BreakRotator (.rotationoffset _item)))
  ;[1 0 0] NOT FIXED FOR REPLICATION: Platform Local Timeline Adjustments
  (CallFunction|StopLocalTimeline)
  (Utilities|FlowControl|Sequence
    (:then_0
      (if (.userotationoffest _item)
        (if (Math|Rotator|Equal(Rotator) (Variables|Default|GetPreviousPlatformRotation) "0, 0, 0" 0.0001)
          (Variables|Default|SetPreviousPlatformRotation (Math|Rotator|MakeRotator (.roll (.rotation _relativeplatformtransform)) (.pitch (.rotation _relativeplatformtransform)) (.yaw (.rotation _relativeplatformtransform)))))
        (Variables|Default|SetNewRotationOffset (Math|Rotator|MakeRotator (+ (.roll (.rotation _relativeplatformtransform)) _roll) (+ (.pitch (.rotation _relativeplatformtransform)) _pitch) (+ (.yaw (.rotation _relativeplatformtransform)) _yaw)))))
    (:then_1
      (if (.uselocationoffset _item)
        (Variables|Default|SetNewLocationOffset (.locationoffset _item))))
    (:then_2
      (Components|Timeline|SetPlayRate (Variables|Default|GetTimeline_1) (.localtimelineplayrate _item))
      (if (== (.maintimelineplayrate _item) 0.0)
        (Components|Timeline|SetPlayRate (Variables|Default|GetTimeline_0) (Variables|Default|GetMainTimelinePlayRate))
        (else
          (Components|Timeline|SetPlayRate (Variables|Default|GetTimeline_0) (.maintimelineplayrate _item)))))
    (:then_3
      (if (or (.userotationoffest _item) (.uselocationoffset _item))
        (CallFunction|StartLocalTimeline)))))

(event Custom|MovePlatformClient
  (bind _targetsplineactor (Variables|Default|GetTargetSplineActor))
  (bind _relativearrowrotation (Variables|Default|GetRelativeArrowRotation))
  (bind _returnvalue (Actor|GetComponentbyClass _targetsplineactor "/Script/Engine.SplineComponent"))
  ;[1 1 1] Main Timeline
  (Utilities|FlowControl|Sequence
    (:then_0
      (bind _movementtimeline (Timeline|Timeline_0 SetNewTime)
        (:Update
          (if (Variables|Default|GetNoTimelineChecks)
            _
            (elif (Variables|Default|GetCompletedAllTimelineChecks)
              _
              (elif (> _movementtimeline (.timelinecheck (Utilities|Array|Get(acopy) (Variables|Default|GetTimelineAdjustments) (Variables|Default|GetTimelineCheckIndex))))
                (CallFunction|ApplyAdjustment)
                (bind _result (Math|Integer|IncrementInt (Variables|Default|GetTimelineCheckIndex))
                  (:%20%20
                    (Variables|Default|SetTimelineCheckIndex _result)
                    (if (== (Utilities|Array|Length (Variables|Default|GetTimelineAdjustments)) (Variables|Default|GetTimelineCheckIndex))
                      (Variables|Default|SetCompletedAllTimelineChecks true)))))))
          (Transformation|SetActorTransform self (Math|Transform|MakeTransform (Spline|GetLocationatDistanceAlongSpline _returnvalue (* (Spline|GetSplineLength _returnvalue) _movementtimeline) "World") (Math|Rotator|MakeRotator (+ (.roll _relativearrowrotation) (.roll (Spline|GetRotationatDistanceAlongSpline _returnvalue (* (Spline|GetSplineLength _returnvalue) _movementtimeline) "World"))) (+ (.pitch _relativearrowrotation) (.pitch (Spline|GetRotationatDistanceAlongSpline _returnvalue (* (Spline|GetSplineLength _returnvalue) _movementtimeline) "World"))) (+ (.yaw _relativearrowrotation) (.yaw (Spline|GetRotationatDistanceAlongSpline _returnvalue (* (Spline|GetSplineLength _returnvalue) _movementtimeline) "World"))))))
          (if (Networking|IsServer)
            (Variables|Default|SetCurrentTimeLinePos _movementtimeline)))
        (:Finished
          (CallFunction|StopLocalTimeline)
          (Variables|Default|SetTimelineCheckIndex 0)
          (Variables|Default|SetCompletedAllTimelineChecks false)
          (Variables|Default|SetPreviousPlatformRotation "0, 0, 0")
          (Variables|Default|SetNewRotationOffset "0, 0, 0")
          (Components|Timeline|SetPlayRate (Variables|Default|GetTimeline_0) (Variables|Default|GetMainTimelinePlayRate))
          (Transformation|SetRelativeTransform (Variables|Default|GetPlatform) (Variables|Default|GetRelativePlatformTransform) false false)
          (Transformation|SetActorRotation self (Variables|Default|GetRelativeArrowRotation))
          (if (Networking|IsServer)
            (Utilities|FlowControl|Delay (Math|Random|RandomFloatinRange (Variables|Default|GetRandomDelayBeforeResetMin) (Variables|Default|GetRandomDelayBeforeResetMax)))
            (Variables|Default|SetCurrentTimeLinePos 0.0)
            (bind _output_get (Variables|Default|SetCurrentRunCounter (+ (Variables|Default|GetCurrentRunCounter) 1)))
            (CallFunction|MulticastStartMovePlatform _output_get)))))
    (:then_1
      (Timeline|Timeline_0 Play))))

(event Custom|StopLocalTimeline
  ;[1 0 0] NOT FIXED FOR REPLICATION: Platform Local Timeline Adjustments
  (Utilities|FlowControl|Sequence
    (:then_0
      (bind _newtrack_0 (Timeline|Timeline_1 Stop)
        (:Update
          (Transformation|SetRelativeTransform (Variables|Default|GetPlatform) (Math|Transform|MakeTransform "0, 0, 0" (Math|Rotator|MakeRotator (.roll (Math|Interpolation|RInterpTo (Variables|Default|GetPreviousPlatformRotation) (Variables|Default|GetNewRotationOffset) _newtrack_0 1.0)) (.pitch (Math|Interpolation|RInterpTo (Variables|Default|GetPreviousPlatformRotation) (Variables|Default|GetNewRotationOffset) _newtrack_0 1.0)) (.yaw (Math|Interpolation|RInterpTo (Variables|Default|GetPreviousPlatformRotation) (Variables|Default|GetNewRotationOffset) _newtrack_0 1.0))) (Transformation|GetWorldScale (Variables|Default|GetPlatform))) false false)
          (if (Networking|IsServer)
            (Variables|Default|SetCurrentLocalTimelinePosition _newtrack_0)))
        (:Finished
          (Variables|Default|SetPreviousPlatformRotation (.Rotation (Math|Transform|BreakTransform (Math|Transform|MakeTransform "0, 0, 0" (Math|Rotator|MakeRotator (.roll (Math|Interpolation|RInterpTo (Variables|Default|GetPreviousPlatformRotation) (Variables|Default|GetNewRotationOffset) _newtrack_0 1.0)) (.pitch (Math|Interpolation|RInterpTo (Variables|Default|GetPreviousPlatformRotation) (Variables|Default|GetNewRotationOffset) _newtrack_0 1.0)) (.yaw (Math|Interpolation|RInterpTo (Variables|Default|GetPreviousPlatformRotation) (Variables|Default|GetNewRotationOffset) _newtrack_0 1.0))) (Transformation|GetWorldScale (Variables|Default|GetPlatform))))) :!label _label))))
    (:then_1
      (goto _label))))

(event Custom|MulticastDrawServerPos
  (params (NewParam :type Transform))
  (bind _platform (Variables|Default|GetPlatform))
  (bind (_min _max) (Components|StaticMesh|GetLocalBounds _platform))
  ;[1 1 1] Debug
  (Rendering|Debug|DrawDebugSphere (.location NewParam) 3e+01 12 "(R=0.015686,G=1.000000,B=0.000000,A=1.000000)" 3.0 2.0)
  (Rendering|Debug|DrawDebugBox (.location NewParam) (/ (- _max _min) 2.0) "(R=0.015686,G=1.000000,B=0.000000,A=1.000000)" (.rotation NewParam) 0.0 2.0))

(event Custom|MulticastStartMovePlatform
  (params (NewCurrentRunCounter :type Integer))
  (bind _targetsplineactor (Variables|Default|GetTargetSplineActor))
  (bind _relativearrowrotation (Variables|Default|GetRelativeArrowRotation))
  (bind _returnvalue (Actor|GetComponentbyClass _targetsplineactor "/Script/Engine.SplineComponent"))
  ;[1 1 1] Main Timeline
  (Variables|Default|SetLastReceivedRunCounter NewCurrentRunCounter)
  (bind _movementtimeline (Timeline|Timeline_0 PlayFromStart)
    (:Update
      (if (Variables|Default|GetNoTimelineChecks)
        _
        (elif (Variables|Default|GetCompletedAllTimelineChecks)
          _
          (elif (> _movementtimeline (.timelinecheck (Utilities|Array|Get(acopy) (Variables|Default|GetTimelineAdjustments) (Variables|Default|GetTimelineCheckIndex))))
            (CallFunction|ApplyAdjustment)
            (bind _result (Math|Integer|IncrementInt (Variables|Default|GetTimelineCheckIndex))
              (:%20%20
                (Variables|Default|SetTimelineCheckIndex _result)
                (if (== (Utilities|Array|Length (Variables|Default|GetTimelineAdjustments)) (Variables|Default|GetTimelineCheckIndex))
                  (Variables|Default|SetCompletedAllTimelineChecks true)))))))
      (Transformation|SetActorTransform self (Math|Transform|MakeTransform (Spline|GetLocationatDistanceAlongSpline _returnvalue (* (Spline|GetSplineLength _returnvalue) _movementtimeline) "World") (Math|Rotator|MakeRotator (+ (.roll _relativearrowrotation) (.roll (Spline|GetRotationatDistanceAlongSpline _returnvalue (* (Spline|GetSplineLength _returnvalue) _movementtimeline) "World"))) (+ (.pitch _relativearrowrotation) (.pitch (Spline|GetRotationatDistanceAlongSpline _returnvalue (* (Spline|GetSplineLength _returnvalue) _movementtimeline) "World"))) (+ (.yaw _relativearrowrotation) (.yaw (Spline|GetRotationatDistanceAlongSpline _returnvalue (* (Spline|GetSplineLength _returnvalue) _movementtimeline) "World"))))))
      (if (Networking|IsServer)
        (Variables|Default|SetCurrentTimeLinePos _movementtimeline)))
    (:Finished
      (CallFunction|StopLocalTimeline)
      (Variables|Default|SetTimelineCheckIndex 0)
      (Variables|Default|SetCompletedAllTimelineChecks false)
      (Variables|Default|SetPreviousPlatformRotation "0, 0, 0")
      (Variables|Default|SetNewRotationOffset "0, 0, 0")
      (Components|Timeline|SetPlayRate (Variables|Default|GetTimeline_0) (Variables|Default|GetMainTimelinePlayRate))
      (Transformation|SetRelativeTransform (Variables|Default|GetPlatform) (Variables|Default|GetRelativePlatformTransform) false false)
      (Transformation|SetActorRotation self (Variables|Default|GetRelativeArrowRotation))
      (if (Networking|IsServer)
        (Utilities|FlowControl|Delay (Math|Random|RandomFloatinRange (Variables|Default|GetRandomDelayBeforeResetMin) (Variables|Default|GetRandomDelayBeforeResetMax)))
        (Variables|Default|SetCurrentTimeLinePos 0.0)
        (bind _output_get (Variables|Default|SetCurrentRunCounter (+ (Variables|Default|GetCurrentRunCounter) 1)))
        (CallFunction|MulticastStartMovePlatform _output_get)))))

(event Custom|StartLocalTimeline
  ;[1 0 0] NOT FIXED FOR REPLICATION: Platform Local Timeline Adjustments
  (bind _newtrack_0 (Timeline|Timeline_1 PlayFromStart)
    (:Update
      (Transformation|SetRelativeTransform (Variables|Default|GetPlatform) (Math|Transform|MakeTransform "0, 0, 0" (Math|Rotator|MakeRotator (.roll (Math|Interpolation|RInterpTo (Variables|Default|GetPreviousPlatformRotation) (Variables|Default|GetNewRotationOffset) _newtrack_0 1.0)) (.pitch (Math|Interpolation|RInterpTo (Variables|Default|GetPreviousPlatformRotation) (Variables|Default|GetNewRotationOffset) _newtrack_0 1.0)) (.yaw (Math|Interpolation|RInterpTo (Variables|Default|GetPreviousPlatformRotation) (Variables|Default|GetNewRotationOffset) _newtrack_0 1.0))) (Transformation|GetWorldScale (Variables|Default|GetPlatform))) false false)
      (if (Networking|IsServer)
        (Variables|Default|SetCurrentLocalTimelinePosition _newtrack_0)))
    (:Finished
      (Variables|Default|SetPreviousPlatformRotation (.Rotation (Math|Transform|BreakTransform (Math|Transform|MakeTransform "0, 0, 0" (Math|Rotator|MakeRotator (.roll (Math|Interpolation|RInterpTo (Variables|Default|GetPreviousPlatformRotation) (Variables|Default|GetNewRotationOffset) _newtrack_0 1.0)) (.pitch (Math|Interpolation|RInterpTo (Variables|Default|GetPreviousPlatformRotation) (Variables|Default|GetNewRotationOffset) _newtrack_0 1.0)) (.yaw (Math|Interpolation|RInterpTo (Variables|Default|GetPreviousPlatformRotation) (Variables|Default|GetNewRotationOffset) _newtrack_0 1.0))) (Transformation|GetWorldScale (Variables|Default|GetPlatform)))))))))

(event Custom|CustomEvent
  (for _array_element (Utilities|Array|MakeArray (Variables|Default|GetSk_male_chest) (Variables|Default|GetSK_male_shoes) (Variables|Default|GetSK_male_head) (Variables|Default|GetSK_male_helmet) (Variables|Default|GetSk_male_bottom) (Variables|Default|GetSk_male_bracers))
    (Class|SkinnedMeshComponent|SetMasterPoseComponent _array_element (Variables|Default|GetSkeletalMesh))
    (Variables|Default|SetRelativeArrowRotation (Variables|/Script/Engine.SceneComponent|GetRelativeRotation (Variables|Default|GetArrow)))
    (Variables|Default|SetRelativePlatformTransform (Transformation|GetRelativeTransform (Variables|Default|GetPlatform)))
    (if (Networking|IsServer)
      (Utilities|FlowControl|Delay (Math|Random|RandomFloatinRange (Variables|Default|GetRandomDelayBeforeStartMin) (Variables|Default|GetRandomDelayBeforeStartMax)))
      (Components|StaticMesh|SetStaticMesh (Variables|Default|GetPlatform) (Variables|Default|GetMesh))
      (Components|Timeline|SetPlayRate (Variables|Default|GetTimeline_0) (Variables|Default|GetMainTimelinePlayRate))
      (if (> (Utilities|Array|Length (Variables|Default|GetTimelineAdjustments)) 0)
        (Variables|Default|SetNoTimelineChecks false))
      (CallFunction|MovePlatform)
      (else
        (Components|Timeline|SetPlayRate (Variables|Default|GetTimeline_0) (Variables|Default|GetMainTimelinePlayRate))
        (if (> (Utilities|Array|Length (Variables|Default|GetTimelineAdjustments)) 0)
          (Variables|Default|SetNoTimelineChecks false))))))

(event Collision|EventActorBeginOverlap
  (params (OtherActor :type Actor%20Object%20Reference)))

(event EventTick
  (params (DeltaSeconds :type Float%20%28single-precision%29)))

(event EventBeginPlay
  (for _array_element (Utilities|Array|MakeArray (Variables|Default|GetSk_male_chest) (Variables|Default|GetSK_male_shoes) (Variables|Default|GetSK_male_head) (Variables|Default|GetSK_male_helmet) (Variables|Default|GetSk_male_bottom) (Variables|Default|GetSk_male_bracers))
    (Class|SkinnedMeshComponent|SetMasterPoseComponent _array_element (Variables|Default|GetSkeletalMesh))
    (Variables|Default|SetRelativeArrowRotation (Variables|/Script/Engine.SceneComponent|GetRelativeRotation (Variables|Default|GetArrow)))
    (Variables|Default|SetRelativePlatformTransform (Transformation|GetRelativeTransform (Variables|Default|GetPlatform)))
    (if (Networking|IsServer)
      (Utilities|FlowControl|Delay (Math|Random|RandomFloatinRange (Variables|Default|GetRandomDelayBeforeStartMin) (Variables|Default|GetRandomDelayBeforeStartMax)))
      (Components|StaticMesh|SetStaticMesh (Variables|Default|GetPlatform) (Variables|Default|GetMesh))
      (Components|Timeline|SetPlayRate (Variables|Default|GetTimeline_0) (Variables|Default|GetMainTimelinePlayRate))
      (if (> (Utilities|Array|Length (Variables|Default|GetTimelineAdjustments)) 0)
        (Variables|Default|SetNoTimelineChecks false))
      (CallFunction|MovePlatform)
      (else
        (Components|Timeline|SetPlayRate (Variables|Default|GetTimeline_0) (Variables|Default|GetMainTimelinePlayRate))
        (if (> (Utilities|Array|Length (Variables|Default|GetTimelineAdjustments)) 0)
          (Variables|Default|SetNoTimelineChecks false))))))

(fn ConstructionScript
  (Components|StaticMesh|SetStaticMesh (Variables|Default|GetPlatform) (Variables|Default|GetMesh)))

(fn OnRepCurrentTimeLinePos
  (bind _currentruncounter (Variables|Default|GetCurrentRunCounter))
  (if (< (Variables|Default|GetLastReceivedRunCounter) _currentruncounter)
    (Variables|Default|SetLastReceivedRunCounter _currentruncounter)
    (CallFunction|MovePlatformClient)))

(fn OnRepCurrentRunCounter
  (bind _currentruncounter (Variables|Default|GetCurrentRunCounter))
  (if (< (Variables|Default|GetLastReceivedRunCounter) _currentruncounter)
    (Variables|Default|SetLastReceivedRunCounter _currentruncounter)
    (CallFunction|MovePlatformClient)))

(fn OnRepCurrentLocalTimelinePosition
  (bind _currentruncounter (Variables|Default|GetCurrentRunCounter))
  (if (< (Variables|Default|GetLastReceivedRunCounter) _currentruncounter)
    (Variables|Default|SetLastReceivedRunCounter _currentruncounter)
    (CallFunction|StartLocalTimelineClient)))

(fn OnRepRepUpdateMovement
  (bind _output_get (Variables|Default|SetUpdateMovement (Variables|Default|GetRep_UpdateMovement)))
  (if _output_get
    (Actor|Tick|SetActorTickEnabled true)))

(fn OnRepRepReverseMovement
  (Variables|Default|SetReverseMovement (Variables|Default|GetRep_ReverseMovement)))

(fn OnRepRepCurrentTimePos
  (bind _output_get (Variables|Default|SetCurrentTimePos (Variables|Default|GetRep_CurrentTimePos)))
  (Variables|Default|SetCurrentTime (* _output_get (Variables|Default|GetMovementDuration))))

(fn OnRepRepVariableRepUpdateTrigger
  ;[1 1 1] These might have been updated locally on the client
  (CallFunction|OnRepRepCurrentTimePos)
  (CallFunction|OnRepRepUpdateMovement))