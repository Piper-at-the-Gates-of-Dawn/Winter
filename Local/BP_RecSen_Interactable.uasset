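; Configurable Conan interactable that, when triggered by interaction, overlap, damage or script, moves or rotates, plays sounds and teaches feats.
; Activation can require and consume an item, and can self-reset after movement.
; Completed moves send integers to a linked instance, which checks ordered or unordered combinations to start itself or reset its senders.
; Movement lerps on a Tick enabled only while moving, using multicast and RepNotify variables for sync.
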(event OnComponentBeginOverlap(TriggerBox)
  (params (OverlappedComponent :type Primitive%20Component%20Object%20Reference) (OtherActor :type Actor%20Object%20Reference) (OtherComp :type Primitive%20Component%20Object%20Reference) (OtherBodyIndex :type Integer) (bFromSweep :type Boolean) (SweepResult :type Hit%20Result%20Structure%20%28by%20ref%29))
  (bind _returnvalue (Actor|GetComponentbyClass OtherActor "/Game/Systems/Components/PlayerNotificationComponent.PlayerNotificationComponent_C"))
  ;[1 1 1] Interaction Trigger
  (if (Utilities|DoesObjectImplementInterface OtherActor "/Game/Systems/Interfaces/BasePlayerCharInterface.BasePlayerCharInterface_C")
    (if (Variables|Default|GetIsInteractionTrigger)
      (if (not (Variables|/Game/Systems/Components/PlayerNotificationComponent.PlayerNotificationComponent_C|GetInteractNotificationCooldownInProgress _returnvalue))
        (Variables|/Game/Systems/Components/PlayerNotificationComponent.PlayerNotificationComponent_C|SetInteractNotificationCooldownInProgress _returnvalue true)
        (bind _asconan_character (Utilities|Casting|CastToConanCharacter OtherActor))
        (bind _isremoteactor (CallFunction|IsRemoteActor _asconan_character))
        (if (not _isremoteactor)
          (CallFunction|ClientShowNotification _asconan_character)
          (Default|StartInteractNotificationCooldown _returnvalue)))
      (elif (not (Variables|Movement(Private)|GetUpdateMovement))
        (if (Variables|Default|GetSelfResetInteractable)
          (if (not (Variables|Default|GetOnCooldown))
            (Variables|Default|SetOnCooldown true)
            (CallFunction|MulticastStartMovement :!label _label)
            (CallFunction|LearnFeat (stale EventInteractableActivate Instigator))
            (if (and (not (Variables|InteractableRotation|GetUseRotationAdjustment)) (not (Variables|InteractableLocation|GetUseLocationAdjustment)))
              (Variables|Default|SetOnCooldown false)))
          (else
            (goto _label)))))))

(event OnComponentBeginOverlap(SafetyTriggerBox)
  (params (OverlappedComponent :type Primitive%20Component%20Object%20Reference) (OtherActor :type Actor%20Object%20Reference) (OtherComp :type Primitive%20Component%20Object%20Reference) (OtherBodyIndex :type Integer) (bFromSweep :type Boolean) (SweepResult :type Hit%20Result%20Structure%20%28by%20ref%29))
  ;[1 1 1] Interaction Trigger
  (if (Variables|Default|GetUseSafetyTriggerBox)
    (if (Utilities|DoesObjectImplementInterface OtherActor "/Game/Systems/Interfaces/BasePlayerCharInterface.BasePlayerCharInterface_C")
      (if (not (Variables|Movement(Private)|GetUpdateMovement))
        (if (Variables|Default|GetSelfResetInteractable)
          (if (not (Variables|Default|GetOnCooldown))
            (Variables|Default|SetOnCooldown true)
            (CallFunction|MulticastStartMovement :!label _label)
            (CallFunction|LearnFeat (stale EventInteractableActivate Instigator))
            (if (and (not (Variables|InteractableRotation|GetUseRotationAdjustment)) (not (Variables|InteractableLocation|GetUseLocationAdjustment)))
              (Variables|Default|SetOnCooldown false)))
          (else
            (goto _label)))))))

(event Custom|ClientShowNotification
  (params (Character :type Conan%20Character%20Object%20Reference))
  (bind _returnvalue (Game|GetPlayerController 0))
  (bind _asbase_hudinterface (Utilities|Casting|CastToBaseHUDInterface (HUD|GetHUD _returnvalue)))
  (bind _returnvalue_2 (UserInterface|CreateWidget "/Game/UI/HUD/Notifications/W_ActionTutorial.W_ActionTutorial_C" _returnvalue))
  (Class|ActionTutorial|CreateActionTutorial _returnvalue_2 "PRESS {0} TO INTERACT" "InteractKey")
  (Class|ActionTutorial|SetFont _returnvalue_2 (Utilities|Struct|MakeSlateFontInfo "/Game/Slate/KelsonSans.KelsonSans" 0 "(OutlineSize=0,OutlineMaterial=None,OutlineColor=(R=0.000000,G=0.000000,B=0.000000,A=1.000000),bSeparateFillAlpha=False)" "Normal" 16))
  (Default|ShowCustomWidgetNotification _asbase_hudinterface _returnvalue_2))

(event Custom|BreakRandomOrderSequence
  (bind _intlistchecker (Variables|InteractableValues|GetIntListChecker))
  ;[1 1 1] Random order sequence
  (Utilities|Array|ForEachLoopwithBreak (Variables|InteractableValues|GetIntListInteraction)) ; enters at Break
)

(event Custom|Break1to1Sequence
  ;[1 1 1] 1 to 1 Sequence
  (Utilities|Array|ForEachLoopwithBreak (Variables|InteractableValues|GetIntListInteraction)) ; enters at Break
)

(event Custom|Add%20value%20to%20triggered%20blueprint
  (bind _blueprint_to_trigger (Variables|InteractableValues|GetBlueprint%20to%20trigger))
  ;[1 1 1] Send values to linked blueprint
  (bind _asbp_rec_sen_interactable (Utilities|Casting|CastToBP_RecSen_Interactable _blueprint_to_trigger))
  (Default|ActorTriggered1 _asbp_rec_sen_interactable _blueprint_to_trigger self (Variables|InteractableValues|GetInt%20Send%20Value%201)))

(event Custom|LearnFeat
  (params (Player%20Controller%20Ref :type Player%20Controller%20Object%20Reference))
  ;[1 1 1] Learn Feat if interacted with
  (for _array_element (Variables|Default|GetFeatId)
    (bind _asconan_character (Utilities|Casting|CastToConanCharacter (Pawn|GetControlledPawn Player%20Controller%20Ref)))
    (bind _returnvalue (Class|ConanCharacter|GetProgressionSystem _asconan_character))
    (Class|ProgressionSystem|ServerForceLearnFeat _returnvalue _array_element true)
    (Variables|Default|SetLearnedAtLeastOneRecipe true))
  ;;[1 1 1] Should check if the player already has the recipe before triggering FIFO
  (if (Variables|Default|GetLearnedAtLeastOneRecipe)
    (Class|ConanCharacter|ClientHUDShowNotification _asconan_character (Variables|Default|GetFIFO%20Text) false)
    (Variables|Default|SetLearnedAtLeastOneRecipe false)))

(event Custom|MulticastPlayAudio
  ;[1 1 1] Play Audio
  (if (Variables|Default|GetResetting)
    (Audio|PlaySoundatLocation (Variables|Audio|GetSoundOnLocationReset) (Transformation|GetWorldLocation (Variables|Default|GetStaticMesh)))
    (else
      (Audio|PlaySoundatLocation (Variables|Audio|GetSoundOnLocation) (Transformation|GetWorldLocation (Variables|Default|GetStaticMesh)))))
  (if (not (Networking|IsDedicatedServer))
    (Audio|PlaySound2D (Variables|Audio|GetSound%202D))))

(event Custom|Check%20pattern
  (bind _intlist (Variables|InteractableValues|GetIntList))
  (if (Variables|InteractableValues|GetSequenceMustBeInCorrectOrder)
    ;[1 1 1] 1 to 1 Sequence
    (bind (_array_element _array_index) (Utilities|Array|ForEachLoopwithBreak (Variables|InteractableValues|GetIntListInteraction))
      (:LoopBody
        (if (== _array_element (Utilities|Array|Get(acopy) (Variables|InteractableValues|GetIntList) _array_index))
          (Variables|InteractableValues|SetIntListSuccess true)
          (else
            (Variables|InteractableValues|SetIntListSuccess false)
            (CallFunction|Break1to1Sequence))))
      (:Completed
        (if (Variables|InteractableValues|GetIntListSuccess)
          (CallFunction|StartSequence)
          (else
            ;[1 1 1] Reset if failure
            (CallFunction|ResetBlueprints)))))
    (else
      ;[1 1 1] Random order sequence
      (Variables|InteractableValues|SetIntListChecker _intlist)
      (bind _array_element_2 (Utilities|Array|ForEachLoopwithBreak (Variables|InteractableValues|GetIntListInteraction))
        (:LoopBody
          (bind (_array_element_3 _array_index_2) (Utilities|Array|ForEachLoopwithBreak _intlist :!label _label)
            (:LoopBody
              (if (== _array_element_2 _array_element_3)
                (if (!= (Utilities|Array|Get(acopy) (Variables|InteractableValues|GetIntListChecker) _array_index_2) -1)
                  (Utilities|Array|SetArrayElem (Variables|InteractableValues|GetIntListChecker) _array_index_2 -1)
                  (Variables|InteractableValues|SetIntListRandomSequenceHit true)
                  (goto _label Break))))
            (:Completed
              (if (Variables|InteractableValues|GetIntListRandomSequenceHit)
                (Variables|InteractableValues|SetIntListRandomSequenceHit false)
                (Variables|InteractableValues|SetIntListSuccess true)
                (else
                  (Variables|InteractableValues|SetIntListRandomSequenceHit false)
                  (Variables|InteractableValues|SetIntListSuccess false)
                  (CallFunction|BreakRandomOrderSequence))))))
        (:Completed
          (if (Variables|InteractableValues|GetIntListSuccess)
            (CallFunction|StartSequence)
            (else
              ;[1 1 1] Reset if failure
              (CallFunction|ResetBlueprints))))))))

(event Custom|StartSequence
  ;[1 1 1] Interaction Trigger
  (if (not (Variables|Movement(Private)|GetUpdateMovement))
    (if (Variables|Default|GetSelfResetInteractable)
      (if (not (Variables|Default|GetOnCooldown))
        (Variables|Default|SetOnCooldown true)
        (CallFunction|MulticastStartMovement :!label _label)
        (CallFunction|LearnFeat (stale EventInteractableActivate Instigator))
        (if (and (not (Variables|InteractableRotation|GetUseRotationAdjustment)) (not (Variables|InteractableLocation|GetUseLocationAdjustment)))
          (Variables|Default|SetOnCooldown false)))
      (else
        (goto _label)))))

(event Custom|ResetBlueprints
  ;[1 1 1] Reset Values
  (for _array_element (Variables|InteractableValues|GetReferencedActors)
    (bind _asbp_rec_sen_interactable (Utilities|Casting|CastToBP_RecSen_Interactable _array_element))
    (Default|ResetTrigger _asbp_rec_sen_interactable _array_element))
  (CallFunction|CleanupInteractionValues))

(event Custom|ResetToReversePosition
  ;[1 1 1] Interaction Trigger
  (if (Variables|Default|GetResetting)
    (CallFunction|MulticastStartMovement)
    (CallFunction|LearnFeat (stale EventInteractableActivate Instigator))
    (if (and (not (Variables|InteractableRotation|GetUseRotationAdjustment)) (not (Variables|InteractableLocation|GetUseLocationAdjustment)))
      (Variables|Default|SetOnCooldown false))))

(event Custom|CleanupInteractionValues
  ;[1 1 1] Reset Values
  (Utilities|Array|Clear (Variables|InteractableValues|GetIntListInteraction))
  (Variables|InteractableValues|SetIntListSuccess false)
  (Utilities|Array|Clear (Variables|InteractableValues|GetReferencedActors)))

(event Custom|CheckForItem
  (params (Player%20controller :type Player%20Controller%20Object%20Reference))
  (bind _returnvalue (Pawn|GetControlledPawn Player%20controller))
  (bind _itemrequired (Variables|ItemRequired|GetItemRequired))
  ;[1 1 1] Item Required
  (if (Class|ItemInventory|HasItembyTemplateID (Class|ItemInventory|GetInventorybyType _returnvalue "Backpack") _itemrequired 1)
    (if (Variables|ItemRequired|GetRemoveItemFromPlayerWhenUsed)
      (bind _success (CallFunction|DeleteItemsinAllInventoriesbyTemplateID Player%20controller _itemrequired 1))
      (bind _asconan_character (Utilities|Casting|CastToConanCharacter _returnvalue))
      (bind _itemname (CallFunction|GetItemName (Variables|ItemRequired|GetItemRequired)))
      (Class|ConanCharacter|ClientHUDShowNotification _asconan_character (Utilities|Text|FormatText "{Text} removed from inventory" _itemname) _success))
    (CallFunction|StartSequence)
    (else
      (bind _asconan_character_2 (Utilities|Casting|CastToConanCharacter _returnvalue))
      (bind _itemname_2 (CallFunction|GetItemName (Variables|ItemRequired|GetItemRequired)))
      (Class|ConanCharacter|ClientHUDShowNotification _asconan_character_2 (Utilities|Text|FormatText "{Text} required" _itemname_2) false))))

(event Custom|TriggeredObjectActionComplete
  ;[1 1 1] Reset when cooldown is finished
  (if (Variables|Default|GetResetAfterTriggerActionsAreFinished)
    (if (Variables|Default|GetSelfResetInteractable)
      (if (Variables|Default|GetResetting)
        (Variables|Default|SetResetting false)
        (Variables|Default|SetOnCooldown false)
        (if (Variables|InteractableValues|GetIntListSuccess)
          (CallFunction|ResetBlueprints))
        (else
          (Variables|Default|SetResetting true)
          (CallFunction|ResettoReversePosition)))
      (else
        (Variables|Default|SetOnCooldown false)))))

(event Custom|InitiateReset
  ;[1 1 1] Reset when cooldown is finished
  (if (Variables|Default|GetResetAfterTriggerActionsAreFinished)
    (if (Variables|Default|GetResetting)
      (if (Variables|Default|GetSelfResetInteractable) :!label _label
        (if (Variables|Default|GetResetting)
          (Variables|Default|SetResetting false)
          (Variables|Default|SetOnCooldown false)
          (if (Variables|InteractableValues|GetIntListSuccess)
            (CallFunction|ResetBlueprints))
          (else
            (Variables|Default|SetResetting true)
            (CallFunction|ResettoReversePosition)))
        (else
          (Variables|Default|SetOnCooldown false))))
    (elif (Variables|Default|GetResetting)
      (goto _label)
      (else
        (Utilities|FlowControl|Delay (Variables|Default|GetResetCooldown))
        (goto _label)))))

(event Custom|MulticastStartMovement
  ;[1 1 1] Start movement/rotation
  (Actor|Tick|SetActorTickEnabled true)
  (Variables|Movement(Private)|SetUpdateMovement true)
  (Variables|Movement(Private)|SetCurrentTime 0.0)
  (Variables|Movement(Private)|SetCurrentTimePos 0.0)
  (CallFunction|MulticastPlayAudio)
  (CallFunction|ReplicateVariables))

(event Custom|MulticastImpactSound
  (Audio|PlaySoundatLocation (Variables|Audio|GetImpactSoundOnLocation) (Transformation|GetWorldLocation (Variables|Default|GetStaticMesh))))

(event EventBeginPlay
  (bind _self self)
  (bind _triggerbox (Variables|Default|GetTriggerBox))
  (for _array_element (Utilities|Array|MakeArray (Variables|Default|GetHead) (Variables|Default|GetFeet) (Variables|Default|GetHelmet) (Variables|Default|GetLeggings) (Variables|Default|GetChest) (Variables|Default|GetBracers))
    (Class|SkinnedMeshComponent|SetMasterPoseComponent _array_element (Variables|Default|GetMasterPoseComponent))
    (for _array_element_2 (Utilities|Array|MakeArray (Variables|Default|GetSkeletalMeshHead) (Variables|Default|GetSkeletalMeshSandals) (Variables|Default|GetSkeletalMeshHelmet) (Variables|Default|GetSkeletalMeshBottom) (Variables|Default|GetSkeletalMeshChest) (Variables|Default|GetSkeletalMeshBracers))
      (Class|SkinnedMeshComponent|SetMasterPoseComponent _array_element_2 (Variables|Default|GetSkeletalMeshMasterPose))
      ;[0.45 1 0.3694] BeginPlay
      (Variables|Default|SetOriginalLocation (Transformation|GetActorLocation _self))
      (if (Variables|InteractableRotation|GetRotateRelativeToParent)
        (Variables|Default|SetOriginalRotation (.Rotation (Math|Transform|BreakTransform (Transformation|GetRelativeTransform (Variables|Default|GetRoot self)))))
        (else
          (Variables|Default|SetOriginalRotation (Transformation|GetActorRotation _self))))
      (if (Variables|Default|GetIsOverlapTrigger)
        (if (Networking|IsServer)
          (Variables|/Script/Engine.PrimitiveComponent|SetbGenerateOverlapEvents _triggerbox true)
          (else
            (Variables|/Script/Engine.PrimitiveComponent|SetbGenerateOverlapEvents _triggerbox false :!label _label)))
        (else
          (goto _label))))))

(event Game|Damage|EventAnyDamage
  (params (Damage :type Float%20%28single-precision%29) (DamageType :type Damage%20Type%20Object%20Reference) (InstigatedBy :type Controller%20Object%20Reference) (DamageCauser :type Actor%20Object%20Reference) (DamageEventID :type Integer))
  ;[1 1 1] Interaction Trigger
  (if (Variables|Default|GetCanTriggerOnDamage)
    (CallFunction|MulticastImpactSound)
    (if (not (Variables|Movement(Private)|GetUpdateMovement))
      (if (Variables|Default|GetSelfResetInteractable)
        (if (not (Variables|Default|GetOnCooldown))
          (Variables|Default|SetOnCooldown true)
          (CallFunction|MulticastStartMovement :!label _label)
          (CallFunction|LearnFeat (stale EventInteractableActivate Instigator))
          (if (and (not (Variables|InteractableRotation|GetUseRotationAdjustment)) (not (Variables|InteractableLocation|GetUseLocationAdjustment)))
            (Variables|Default|SetOnCooldown false)))
        (else
          (goto _label))))))

(event EventInteractableActivate
  (params (Component :type Primitive%20Component%20Object%20Reference) (Instigator :type Player%20Controller%20Object%20Reference) (HitIndex :type Integer) (TriggeredFromRadialWheel :type Boolean))
  ;[1 1 1] Interaction Trigger
  (if (Variables|Default|GetIsInteractionTrigger)
    (if (Variables|ItemRequired|GetRequiresItem)
      (CallFunction|CheckforItem Instigator)
      (elif (not (Variables|Movement(Private)|GetUpdateMovement))
        (if (Variables|Default|GetSelfResetInteractable)
          (if (not (Variables|Default|GetOnCooldown))
            (Variables|Default|SetOnCooldown true)
            (CallFunction|MulticastStartMovement :!label _label)
            (CallFunction|LearnFeat Instigator)
            (if (and (not (Variables|InteractableRotation|GetUseRotationAdjustment)) (not (Variables|InteractableLocation|GetUseLocationAdjustment)))
              (Variables|Default|SetOnCooldown false)))
          (else
            (goto _label)))))))

(event EventResetTrigger
  (params (Actor :type Actor%20Object%20Reference))
  ;[1 1 1] Reset when cooldown is finished
  (if (Variables|Default|GetResetAfterTriggerActionsAreFinished)
    (if (Variables|Default|GetSelfResetInteractable)
      (if (Variables|Default|GetResetting)
        (Variables|Default|SetResetting false)
        (Variables|Default|SetOnCooldown false)
        (if (Variables|InteractableValues|GetIntListSuccess)
          (CallFunction|ResetBlueprints))
        (else
          (Variables|Default|SetResetting true)
          (CallFunction|ResettoReversePosition)))
      (else
        (Variables|Default|SetOnCooldown false)))))

(event EventTick
  (params (DeltaSeconds :type Float%20%28single-precision%29))
  (bind _originalrotation (Variables|Default|GetOriginalRotation))
  (bind _movementduration (Variables|Default|GetMovementDuration))
  (bind _originallocation (Variables|Default|GetOriginalLocation))
  (bind _tempwaterfillingref (Variables|Default|GetTempWaterFillingRef))
  ;[1 1 1] Don't really need this anymore with the ticking being turned on and off
  (if (Variables|Movement(Private)|GetUpdateMovement)
    (Utilities|FlowControl|Sequence
      (:then_0
        (Variables|Movement(Private)|SetCurrentTimePos (/ (Variables|Movement(Private)|GetCurrentTime) (Variables|Default|GetMovementDuration))))
      (:then_1
        ;[1 1 1] Location
        (if (Variables|InteractableLocation|GetUseLocationAdjustment)
          (Transformation|SetActorLocation self (Math|Vector|Lerp(Vector) _originallocation (+ _originallocation (Variables|InteractableLocation|GetLocationAdjustment)) (Math|Float|SelectFloat (- 1.0 (Variables|Movement(Private)|GetCurrentTimePos)) (Variables|Movement(Private)|GetCurrentTimePos) (Variables|Movement(Private)|GetReverseMovement))) false true)))
      (:then_2
        ;[1 1 1] Rotation
        (if (Variables|InteractableRotation|GetUseRotationAdjustment)
          (if (Variables|InteractableRotation|GetRotateRelativeToParent)
            (Transformation|SetActorRelativeRotation (Math|Rotator|Lerp(Rotator) _originalrotation (Math|Rotator|CombineRotators _originalrotation (Variables|InteractableRotation|GetRotationAdjustment)) (Math|Float|SelectFloat (- 1.0 (Variables|Movement(Private)|GetCurrentTimePos)) (Variables|Movement(Private)|GetCurrentTimePos) (Variables|Movement(Private)|GetReverseMovement))))
            (else
              (Transformation|SetActorRotation (Math|Rotator|Lerp(Rotator) _originalrotation (Math|Rotator|CombineRotators _originalrotation (Variables|InteractableRotation|GetRotationAdjustment)) (Math|Float|SelectFloat (- 1.0 (Variables|Movement(Private)|GetCurrentTimePos)) (Variables|Movement(Private)|GetCurrentTimePos) (Variables|Movement(Private)|GetReverseMovement))))))))
      (:then_3
        (bind _output_get (Variables|Movement(Private)|SetCurrentTime (Math|Float|Min(Float) (+ (Variables|Movement(Private)|GetCurrentTime) (Utilities|Time|GetWorldDeltaSeconds)) _movementduration)))
        (if (== _output_get _movementduration)
          (Utilities|FlowControl|Sequence
            (:then_0
              (Variables|Movement(Private)|SetUpdateMovement false)
              (Actor|Tick|SetActorTickEnabled false))
            (:then_1
              (Variables|Movement(Private)|SetReverseMovement (not (Variables|Movement(Private)|GetReverseMovement))))
            (:then_2
              (if (Networking|IsServer)
                (if (Variables|Default|GetSelfResetInteractable)
                  (if (Variables|Default|GetResetting)
                    (CallFunction|InitiateReset)
                    (else
                      (CallFunction|InitiateReset)
                      (if (Networking|IsServer) :!label _label
                        (CallFunction|AddValuetoTriggeredBlueprint))))
                  (else
                    (goto _label)))
                ;[1 1 1] Temp until a proper list system is made
                (if (not (== _tempwaterfillingref 0))
                  (Default|StartSequence _tempwaterfillingref (Variables|InteractableValues|GetFloatValue1) self))))))))))

(event EventActorTriggered1
  (params (Blueprint%20to%20Trigger :type Actor%20Object%20Reference) (BlueprintTriggerer :type Actor%20Object%20Reference) (Int%20Value%201 :type Integer))
  ;[1 1 1] Add values and references to blueprints
  (Utilities|Array|Add (Variables|InteractableValues|GetIntListInteraction) Int%20Value%201)
  (Utilities|Array|Add (Variables|InteractableValues|GetReferencedActors) BlueprintTriggerer)
  (if (== (Utilities|Array|Length (Variables|InteractableValues|GetIntList)) (Utilities|Array|Length (Variables|InteractableValues|GetIntListInteraction)))
    ;;[1 1 1] autocheck trigger
    (if true
      (CallFunction|CheckPattern))))

(event EventTrigger
  (params (Data :type STR%20Trigger%20Message%20Structure))
  (CallFunction|StartSequence))

(fn ConstructionScript
  (bind _texttoshow (Variables|Default|GetTextToShow))
  (bind _textrender2 (Variables|Default|GetTextRender2))
  (bind _textrender (Variables|Default|GetTextRender))
  (bind _textscale (Variables|Default|GetTextScale))
  (bind _textcolor (Variables|Default|GetTextColor))
  (bind _returnvalue (Math|Conversions|ToColor(LinearColor) _textcolor))
  (Rendering|Components|TextRender|SetWorldSize _textrender _textscale)
  (Rendering|Components|TextRender|SetText _textrender _texttoshow)
  (Rendering|Components|TextRender|SetTextRenderColor _textrender _returnvalue)
  (Rendering|Components|TextRender|SetWorldSize _textrender2 _textscale)
  (Rendering|Components|TextRender|SetText _textrender2 _texttoshow)
  (Rendering|Components|TextRender|SetTextRenderColor _textrender2 _returnvalue))

(fn ReplicateVariables
  (if (Networking|IsServer)
    (Variables|Movement(Replication)|SetRep_UpdateMovement (Variables|Movement(Private)|GetUpdateMovement))
    (Variables|Movement(Replication)|SetRep_ReverseMovement (Variables|Movement(Private)|GetReverseMovement))
    (Variables|Movement(Replication)|SetRep_CurrentTimePos (Variables|Movement(Private)|GetCurrentTimePos))
    (Variables|Movement(Replication)|SetRep_VariableRepUpdateTrigger (not (Variables|Movement(Replication)|GetRep_VariableRepUpdateTrigger)))))

(fn OnRepRepUpdateMovement
  (bind _output_get (Variables|Movement(Private)|SetUpdateMovement (Variables|Movement(Replication)|GetRep_UpdateMovement)))
  (if _output_get
    (Actor|Tick|SetActorTickEnabled true)))

(fn OnRepRepReverseMovement
  (Variables|Movement(Private)|SetReverseMovement (Variables|Movement(Replication)|GetRep_ReverseMovement)))

(fn OnRepRepCurrentTimePos
  (bind _output_get (Variables|Movement(Private)|SetCurrentTimePos (Variables|Movement(Replication)|GetRep_CurrentTimePos)))
  (Variables|Movement(Private)|SetCurrentTime (* _output_get (Variables|Default|GetMovementDuration))))

(fn OnRepRepVariableRepUpdateTrigger
  ;[1 1 1] These might have been updated locally on the client
  (CallFunction|OnRepRepCurrentTimePos)
  (CallFunction|OnRepRepUpdateMovement))

(fn GetItemName
  (params (ItemTemplateID :type Integer))
  (bind _returnvalue (Utilities|GetDataTableRow "/Game/Items/ItemTable.ItemTable" (Utilities|String|StringToName (Utilities|String|ToString(Integer) ItemTemplateID)))
    (:then
      (return (.name _returnvalue)))
    (:RowNotFound
      (return ""))))

(fn InteractableActivateDisabled
  (params (InteractingCharacter :type Conan%20Character%20Object%20Reference))
  (return false))

(fn InteractableCanbeLooted
  (params (InteractingCharacter :type Conan%20Character%20Object%20Reference))
  (return false))

(fn InteractableDefaultAction
  (return "" 0))

(fn InteractableGetRepairUIModuleName
  (return "None"))

(fn InteractableGetSimpleDisplayText
  (return "None"))

(fn InteractableGetUIModuleName
  (return "None"))

(fn InteractableMenuDisabled
  (params (InteractingCharacter :type Conan%20Character%20Object%20Reference))
  (return false))

(fn InteractableShouldCommand
  (return false))