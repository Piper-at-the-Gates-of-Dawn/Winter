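; Loot chest placeable for legendary items that needs a key item in the player's backpack to open.
; First opening consumes the key and sets HasBeenOpened, after which interaction works without one.
; Item removal and stat-change signals from its inventory recount the Legendaries list, destroying the chest with a particle effect when none remain.
; An old level-requirement check is left disconnected.
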(event SignalItemRemoved(ItemInventoryReplicateToAll)
  (params (index :type Integer) (item :type Game%20Item%20Object%20Reference) (dstInventory :type Item%20Inventory%20Object%20Reference) (dstIndex :type Integer))
  (if (!= dstInventory (Variables|Default|GetItemInventoryReplicateToAll))
    (Variables|Default|SetCounter 0)
    (for _array_element (Variables|Default|GetLegendaries)
      (bind _resourcecount (CallFunction|GetCompleteResourceCount 0 _array_element))
      (Variables|Default|SetCounter (+ _resourcecount (Variables|Default|GetCounter))))
    (if (< (Variables|Default|GetCounter) 1)
      ;[1 1 1] Spawn a particle to help contexualize the chest disappearing on DestroyActor
      (Effects|SpawnEmitteratLocation 0 (Transformation|GetWorldLocation (Variables|Default|GetSkeletalMesh)))
      (Actor|DestroyActor))))

(event SignalItemAdded(ItemInventoryReplicateToAll)
  (params (index :type Integer) (item :type Game%20Item%20Object%20Reference) (srcInventory :type Item%20Inventory%20Object%20Reference) (srcIndex :type Integer)))

(event SignalItemIntStatChanged(ItemInventoryReplicateToAll)
  (params (item :type Game%20Item%20Object%20Reference) (statID :type EItemIntStatID%20Enum :default "MaxStackSize") (statValue :type Integer) (deltaValue :type Integer))
  (Variables|Default|SetCounter 0)
  (for _array_element (Variables|Default|GetLegendaries)
    (bind _resourcecount (CallFunction|GetCompleteResourceCount 0 _array_element))
    (Variables|Default|SetCounter (+ _resourcecount (Variables|Default|GetCounter))))
  (if (< (Variables|Default|GetCounter) 1)
    ;[1 1 1] Spawn a particle to help contexualize the chest disappearing on DestroyActor
    (Effects|SpawnEmitteratLocation 0 (Transformation|GetWorldLocation (Variables|Default|GetSkeletalMesh)))
    (Actor|DestroyActor)))

(event SignalItemFloatStatChanged(ItemInventoryReplicateToAll)
  (params (item :type Game%20Item%20Object%20Reference) (statID :type EItemFloatStatID%20Enum :default "WeaponStaminaHeavyChargedRegenModifier") (statValue :type Float%20%28single-precision%29) (deltaValue :type Float%20%28single-precision%29))
  (Variables|Default|SetCounter 0)
  (for _array_element (Variables|Default|GetLegendaries)
    (bind _resourcecount (CallFunction|GetCompleteResourceCount 0 _array_element))
    (Variables|Default|SetCounter (+ _resourcecount (Variables|Default|GetCounter))))
  (if (< (Variables|Default|GetCounter) 1)
    ;[1 1 1] Spawn a particle to help contexualize the chest disappearing on DestroyActor
    (Effects|SpawnEmitteratLocation 0 (Transformation|GetWorldLocation (Variables|Default|GetSkeletalMesh)))
    (Actor|DestroyActor)))

(event EventInteractableActivate
  (params (Component :type Primitive%20Component%20Object%20Reference) (Instigator :type Player%20Controller%20Object%20Reference) (HitIndex :type Integer) (TriggeredFromRadialWheel :type Boolean))
  (bind _asconan_character (Utilities|Casting|CastToConanCharacter (Pawn|GetControlledPawn Instigator)))
  (Variables|Default|SetConanCharacterRef _asconan_character)
  (bind _returnvalue (Class|ConanCharacter|GetBackpackInventory (Variables|Default|GetConanCharacterRef)))
  (if (Class|ItemInventory|HasItembyTemplateID _returnvalue (Variables|Default|GetLegendaryChestRequiredItem) 1)
    (|CallParentFunction Component Instigator HitIndex false :!label _label)
    (if (not (Variables|Default|GetHasBeenOpened))
      (bind _returnvalue_2 (Class|ConanCharacter|GetBackpackInventory (Variables|Default|GetConanCharacterRef)))
      (Class|ItemInventory|DeleteItemsbyTemplate _returnvalue_2 (Variables|Default|GetLegendaryChestRequiredItem) 1)
      (Variables|Default|SetHasBeenOpened true))
    (elif (Variables|Default|GetHasBeenOpened)
      (goto _label)
      (else
        (Class|ConanCharacter|ClientHUDShowNotification (Variables|Default|GetConanCharacterRef) (Variables|Default|GetMustHaveKey) false)))))

(fn ConstructionScript
  (|CallParentFunction))